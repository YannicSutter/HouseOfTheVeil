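; Trigger volume that ends the demo and shows the end-of-demo screen.
; Any overlap on its Collision component runs EndDemo while BIsActive is set, with no check on the overlapping actor.
; EndDemo switches the player character's current view enum, removes the movement input mapping context, adds WBP_EndDemoScreen to the viewport, sets its texture and shows the mouse cursor.
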(event `self.Collision.OnComponentBeginOverlap`
  (params (OverlappedComponent :type "PrimitiveComponent Object Reference") (OtherActor :type "Actor Object Reference") (OtherComp :type "PrimitiveComponent Object Reference") (OtherBodyIndex :type Integer) (bFromSweep :type Boolean) (SweepResult :type "HitResult Structure (by ref)"))
  ;[0.15 0 0.001187 0.5] Trigger Logic
  (if (`self.b_isActive`)
    (`self.EndDemo`)))

(event `EndDemo`
  (bind _returnvalue (`GameplayStatics.GetPlayerController` 0))
  ;[0.15 0 0.001187 0.5] Trigger Logic
  (bind _asbp_player_character (cast `/Game/HouseEdwards/Blueprints/PlayerCharacter/BP_PlayerCharacter` (`GameplayStatics.GetPlayerCharacter` 0)))
  (set `/Game/HouseEdwards/Blueprints/PlayerCharacter/BP_PlayerCharacter.enum_currentView` "NewEnumerator6" _asbp_player_character)
  (`EnhancedInputSubsystemInterface.RemoveMappingContext` (pcsubsystem `EnhancedInputLocalPlayerSubsystem` _returnvalue) "/Game/HouseEdwards/Blueprints/PlayerCharacter/Input/IMC_Movement.IMC_Movement" (struct))
  (bind _returnvalue_2 (`|CreateWidget` "/Game/HouseEdwards/Blueprints/UI/WBP_EndDemoScreen.WBP_EndDemoScreen_C" _returnvalue))
  (`UserWidget.AddToViewport` _returnvalue_2 0)
  (`/Game/HouseEdwards/Blueprints/UI/WBP_EndDemoScreen.SetTexture` _returnvalue_2 null)
  (set `PlayerController.bShowMouseCursor` true _returnvalue))

(fn `UserConstructionScript`)