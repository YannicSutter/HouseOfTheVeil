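; Interactive piano puzzle: the player enters a piano camera view and must repeat four melody parts by clicking keys.
; Cursor traces highlight keys through dynamic materials; clicks animate them and play mapped sounds.
; Each part's song data asset drives a recursive, delay-timed demo and note checking (MIDI minus 21 indexes the keys), with UI feedback.
; Completion restores player control and starts final playback; the finished flag's OnRep handles spawning the mother doll.
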(event `self.ReceiveBeginPlay`
  ; Begin Play
  (set `self.b_isPlaying` true)
  (`KismetArrayLibrary.Array_Clear` (`self.a_playedKeyQueue`))
  (set `self.a_playedKeyQueue` (`|MakeArray` null null null null null null :!type "StaticMeshComponent Object Reference")))

(event `self.ReceiveTick`
  (params (DeltaSeconds :type "Float (single-precision)"))
  (bind _sm_currentkey (`self.sm_currentKey`))
  (bind _sm_currentkey_2 (`self.sm_currentKey`))
  (bind (_bblockinghit _binitialoverlap _time _distance _location _impactpoint _normal _impactnormal _physmat _hitactor _hitcomponent) (`GameplayStatics.BreakHitResult` (`PlayerController.GetHitResultUnderCursorByChannel` (`GameplayStatics.GetPlayerController` 0) "TraceTypeQuery1" true)))
  (bind _componenttags (`ActorComponent.ComponentTags` _hitcomponent))
  ;[0.15 0 0.03106 0.5] Interact Logic
  (if (not (`self.b_isPlaying`))
    ;; Interact (same as Chess Puzzle by Yannic)
    (`/Engine/EditorBlueprintResources/StandardMacros.IsValid` _hitcomponent
      (:`Is Valid`
        (if (> (`KismetArrayLibrary.Array_Length` _componenttags) 0)
          (if (== (`|GetArrayItem` _componenttags) "Key")
            (`/Engine/EditorBlueprintResources/StandardMacros.IsValid` _sm_currentkey_2
              (:`Is Valid`
                (`self.HoverUnhighlight` _sm_currentkey_2))
              (:`Is Not Valid`
                _))
            (bind _asstatic_mesh_component (cast `StaticMeshComponent` _hitcomponent))
            (bind _output_get (set `self.sm_currentKey` _asstatic_mesh_component))
            (`self.HoverHighlight` _output_get))
          (elif (!= _sm_currentkey null)
            (`self.HoverUnhighlight` _sm_currentkey)
            (set `self.sm_currentKey` null)))))))

(event `Interact`
  (bind _returnvalue (`GameplayStatics.GetPlayerController` 0))
  (bind _returnvalue_2 (`GameplayStatics.GetPlayerController` 0))
  (bind _returnvalue_3 (pcsubsystem `EnhancedInputLocalPlayerSubsystem` (`GameplayStatics.GetPlayerController` 0)))
  ;[0.15 0 0.03106 0.5] Interact Logic
  ;; E Interact (same as Chess Puzzle by Yannic)
  (bind _asbp_player_character (cast `/Game/HouseEdwards/Blueprints/PlayerCharacter/BP_PlayerCharacter` (`GameplayStatics.GetPlayerCharacter` 0)))
  (if (`|EnumEquality` (`/Game/HouseEdwards/Blueprints/PlayerCharacter/BP_PlayerCharacter.enum_currentView` _asbp_player_character) "NewEnumerator2")
    (set `/Game/HouseEdwards/Blueprints/PlayerCharacter/BP_PlayerCharacter.enum_currentView` "NewEnumerator0" _asbp_player_character)
    ;;; Handling Controls Input
    (`EnhancedInputSubsystemInterface.AddMappingContext` _returnvalue_3 "/Game/HouseEdwards/Blueprints/PlayerCharacter/Input/IMC_Movement.IMC_Movement" 0 (struct))
    (set `PlayerController.bShowMouseCursor` false _returnvalue)
    ;;; Set Camera View
    (`PlayerController.SetViewTargetWithBlend` _returnvalue_2 (`GameplayStatics.GetPlayerCharacter` 0) 2.0 "VTBlend_EaseIn" 3.0 false)
    (bind _sm_currentkey (`self.sm_currentKey`)
      (:`then`
        (`self.HoverUnhighlight` _sm_currentkey))
      (:`else`
        _))
    (`KismetSystemLibrary.Delay` 2.0)
    (set `self.b_isPlaying` true)
    (set `self.sm_currentKey` null)
    (`Widget.RemoveFromParent` (`self.wbp_PianoUI`))
    (`WidgetBlueprintLibrary.SetInputMode_GameOnly` (`GameplayStatics.GetPlayerController` 0))
    (`self.FixKeyRotation`)
    (else
      (set `/Game/HouseEdwards/Blueprints/PlayerCharacter/BP_PlayerCharacter.enum_currentView` "NewEnumerator2" _asbp_player_character)
      (`EnhancedInputSubsystemInterface.RemoveMappingContext` _returnvalue_3 "/Game/HouseEdwards/Blueprints/PlayerCharacter/Input/IMC_Movement.IMC_Movement" (struct))
      (set `PlayerController.bShowMouseCursor` true _returnvalue)
      (`PlayerController.SetViewTargetWithBlend` _returnvalue_2 self 1.0 "VTBlend_EaseIn" 3.0 false)
      (`KismetSystemLibrary.Delay` 2.0)
      (if (`self.b_PuzzleFinished`)
        (set `self.b_isPlaying` false)
        (`WidgetBlueprintLibrary.SetInputMode_GameAndUIEx` (`GameplayStatics.GetPlayerController` 0) null)
        (else
          (`self.PlayPuzzle`)
          (set `self.b_isPlaying` false)
          (bind _returnvalue_4 (`|CreateWidget` "/Game/HouseEdwards/Blueprints/Piano_BP/WBP_Piano_UI.WBP_Piano_UI_C"))
          (bind _output_get (set `self.wbp_PianoUI` _returnvalue_4))
          (`UserWidget.AddToViewport` _output_get 0)
          (`WidgetBlueprintLibrary.SetInputMode_GameAndUIEx` (`GameplayStatics.GetPlayerController` 0) _output_get))))))

(event `HoverHighlight`
  (params (Key :type "StaticMeshComponent Object Reference"))
  ;[0.15 0 0.03106 0.5] Interact Logic
  (bind _asmaterial_instance_dynamic (cast `MaterialInstanceDynamic` (`PrimitiveComponent.GetMaterial` Key 0)))
  (`MaterialInstanceDynamic.SetVectorParameterValue` _asmaterial_instance_dynamic "EmissiveColor" (struct :`R` 0.546875 :`G` 0.277046 :`B` 0.141466 :`A` 1.0)))

(event `HoverUnhighlight`
  (params (Key :type "StaticMeshComponent Object Reference"))
  ;[0.15 0 0.03106 0.5] Interact Logic
  (bind _asmaterial_instance_dynamic (cast `MaterialInstanceDynamic` (`PrimitiveComponent.GetMaterial` Key 0)))
  (`MaterialInstanceDynamic.SetVectorParameterValue` :`self` _asmaterial_instance_dynamic :`ParameterName` "EmissiveColor"))

(event `HandleClick`
  (bind _sm_pressedkey (`self.Sm_pressedKey`))
  (bind _sm_currentkey (`self.sm_currentKey`))
  ; Press Piano Key Logic
  (`/Engine/EditorBlueprintResources/StandardMacros.IsValid` _sm_currentkey
    (:`Is Valid`
      (if (not (`self.b_isPlaying`))
        (set `self.Sm_pressedKey` _sm_currentkey)
        (if (not (`self.b_PuzzleFinished`))
          ;; Check puzzle solution
          (`self.AddToQueue`)
          (`self.CheckPlayedNote`))
        (set `self.b_isPlaying` true)
        ;; Rotate pressed key and play sound
        (`self.MapSoundToKey` _sm_pressedkey)
        (`self.RotateKey` _sm_pressedkey)))))

(event `RotateKey`
  (params (keyToPress :type "StaticMeshComponent Object Reference"))
  ; Press Key Animation
  ;; Piano Key Animation
  (bind _output_get (set `self.t_transform` (`SceneComponent.GetRelativeTransform` keyToPress)))
  (bind (_direction _f_keyangle) (`Timeline|Timeline` :!via `PlayFromStart`)
    (:`Update`
      (bind _output_get_2 (set `self.r_targetRotation` (`KismetMathLibrary.MakeRotator` 0.0 (+ _f_keyangle (.pitch (.rotation _output_get))))))
      (`SceneComponent.K2_SetRelativeRotation` keyToPress _output_get_2 false false))
    (:`Finished`
      (set `self.b_isPlaying` false))))

(event `CheckPlayedNote`
  (bind _wbp_pianoui (`self.wbp_PianoUI`))
  (bind _wbp_pianoui_2 (`self.wbp_PianoUI`))
  ; Check pressed key
  ;; Check Solution
  ;; Check if the right key was played
  (bind _puzzletoplay (`self.ReturnPuzzlePart`))
  (bind _notes (`UPianoSongData.Notes` _puzzletoplay))
  (bind _output_midi (break `NoteEvent` (`|GetArrayItem` _notes (`self.i_corrrectNotesPlayed`))))
  (if (== (`|GetArrayItem` (`self.KeyComponent`) (- _output_midi 21)) (`self.Sm_pressedKey`))
    ;; Visual UI feedback for player
    (bind _output_get (set `self.i_corrrectNotesPlayed` (+ (`self.i_corrrectNotesPlayed`) 1)))
    (`/Game/HouseEdwards/Blueprints/Piano_BP/WBP_Piano_UI.changeColorImage` _wbp_pianoui _output_get)
    (if (== _output_get (`KismetArrayLibrary.Array_Length` _notes))
      (`/Game/HouseEdwards/Blueprints/Piano_BP/WBP_Piano_UI.ShowSuccessText` _wbp_pianoui_2)
      (`KismetSystemLibrary.Delay` 0.5)
      (bind _output_get_2 (set `self.i_corrrectNotesPlayed` 0))
      (`/Game/HouseEdwards/Blueprints/Piano_BP/WBP_Piano_UI.changeColorImage` _wbp_pianoui_2 _output_get_2)
      (bind _output_get_3 (set `self.i_puzzleProgress` (+ (`self.i_puzzleProgress`) 1)))
      ;; Starts sequence if puzzle was completed
      (bind _output_get_4 (set `self.b_PuzzleFinished` (== _output_get_3 4)))
      (if _output_get_4
        (`KismetSystemLibrary.Delay` 2.0)
        (`self.EndPuzzle`)
        ;; Puzzle end animation and piano song
        (`self.StartPlayback`)
        (`KismetSystemLibrary.Delay` 2.0)
        (`GameplayStatics.PlaySoundAtLocation` "/Game/HouseEdwards/Assets/PianoPuzzle/SongDataFiles/sc_House_of_the_Veil_Cue.sc_House_of_the_Veil_Cue" (`self.K2_GetActorLocation`) (struct) 1.0 1.0 0.0 null null null null)
        (else
          (`self.PlayPuzzle`))))
    (else
      (bind _output_get_5 (set `self.i_corrrectNotesPlayed` 0))
      (`/Game/HouseEdwards/Blueprints/Piano_BP/WBP_Piano_UI.changeColorImage` _wbp_pianoui _output_get_5))))

(event `PlayPuzzle`
  ; Puzzle part sequence
  (if (not (`self.b_pianoIsPlaying`))
    (set `self.b_pianoIsPlaying` true)
    (bind _puzzletoplay (`self.ReturnPuzzlePart`))
    (`self.RecursivePianoLoop` 0 (`UPianoSongData.Notes` _puzzletoplay))))

(event `RecursivePianoLoop`
  (params (Index :type Integer) (Notes :type "Array of NoteEvent Structure"))
  (bind _returnvalue (+ Index 1))
  (bind (_midi _time _duration) (break `NoteEvent` (`|GetArrayItem` Notes Index)))
  (bind _output (`|GetArrayItem` (`self.KeyComponent`) (- _midi 21)))
  ; Recursive event to play the notes from the "Song Data Files"
  ;; Play piano solution
  (if (>= Index (- (`KismetArrayLibrary.Array_Length` Notes) 1))
    (`self.MapSoundToKey` _output)
    (`self.RotateKey` _output)
    (`self.HoverHighlight` _output)
    (`KismetSystemLibrary.Delay` _duration)
    (`self.HoverUnhighlight` _output)
    (set `self.b_pianoIsPlaying` false)
    (`self.FixKeyRotation`)
    (else
      (`self.MapSoundToKey` _output)
      (`self.RotateKey` _output)
      (`self.HoverHighlight` _output)
      (`KismetSystemLibrary.Delay` (- (`.Time` (break `NoteEvent` (`|GetArrayItem` Notes _returnvalue))) _time))
      (`self.HoverUnhighlight` _output)
      (`self.RecursivePianoLoop` _returnvalue Notes))))

(event `EndPuzzle`
  ; Puzzle solved end sequence
  (bind _sm_currentkey (`self.sm_currentKey`)
    (:`then`
      (`self.HoverUnhighlight` _sm_currentkey))
    (:`else`
      _))
  (bind _asbp_player_character (cast `/Game/HouseEdwards/Blueprints/PlayerCharacter/BP_PlayerCharacter` (`GameplayStatics.GetPlayerCharacter` 0)))
  (`Widget.RemoveFromParent` (`self.wbp_PianoUI`))
  (`WidgetBlueprintLibrary.SetInputMode_GameOnly` (`GameplayStatics.GetPlayerController` 0))
  (set `/Game/HouseEdwards/Blueprints/PlayerCharacter/BP_PlayerCharacter.enum_currentView` "NewEnumerator0" _asbp_player_character)
  (`EnhancedInputSubsystemInterface.AddMappingContext` (pcsubsystem `EnhancedInputLocalPlayerSubsystem` (`GameplayStatics.GetPlayerController` 0)) "/Game/HouseEdwards/Blueprints/PlayerCharacter/Input/IMC_Movement.IMC_Movement" 0 (struct))
  (set `PlayerController.bShowMouseCursor` false (`GameplayStatics.GetPlayerController` 0))
  (set `self.b_isPlaying` true)
  (`PlayerController.SetViewTargetWithBlend` (`GameplayStatics.GetPlayerController` 0) (`GameplayStatics.GetPlayerCharacter` 0) 5.0 "VTBlend_EaseOut" 4.0 false)
  (`WidgetBlueprintLibrary.SetInputMode_GameOnly` (`GameplayStatics.GetPlayerController` 0))
  (`KismetSystemLibrary.Delay` 2.0))

(fn `AddToQueue`
  (bind _a_playedkeyqueue (`self.a_playedKeyQueue`))
  (if (== (`KismetArrayLibrary.Array_Length` (`self.a_playedKeyQueue`)) 6)
    (`KismetArrayLibrary.Array_Remove` _a_playedkeyqueue)
    (`KismetArrayLibrary.Array_Add` _a_playedkeyqueue (`self.Sm_pressedKey`))
    (else
      (`KismetArrayLibrary.Array_Add` (`self.a_playedKeyQueue`) (`self.Sm_pressedKey`)))))

(fn `FixKeyRotation`
  (for _array_element (`self.KeyComponent`)
    (bind _returnvalue (`SceneComponent.GetRelativeTransform` _array_element))
    (`SceneComponent.K2_SetRelativeRotation` _array_element (`KismetMathLibrary.MakeRotator` (.roll (.rotation _returnvalue)) 0.0 (.yaw (.rotation _returnvalue))) false false)))

(fn `MapSoundToKey`
  (params (keyToPlay :type "StaticMeshComponent Object Reference"))
  (bind (_value _returnvalue) (`BlueprintMapLibrary.Map_Find` (`self.SoundMap`) (`KismetStringLibrary.Conv_StringToName` (`KismetSystemLibrary.GetObjectName` keyToPlay))))
  (if _returnvalue
    (`GameplayStatics.PlaySound2D` _value 1.0 1.0 0.0 null null)
    (else
      (`KismetSystemLibrary.PrintString` "Couldn't map key to sound"))))

(fn `OnRep_b_PuzzleFinished`
  (bind _outactors (`GameplayStatics.GetAllActorsOfClass` "/Game/HouseEdwards/Blueprints/Interactables/BP_Interactable_Doll_Mother.BP_Interactable_Doll_Mother_C"))
  (`/Engine/EditorBlueprintResources/StandardMacros.IsValid` (`|GetArrayItem` _outactors)
    (:`Is Not Valid`
      (`|SpawnActorFromClass` "/Game/HouseEdwards/Blueprints/Interactables/BP_Interactable_Doll_Mother.BP_Interactable_Doll_Mother_C" (`KismetMathLibrary.MakeTransform` (-349.803258 -1134.702375 54.371578) (struct :`Pitch` 1.289923 :`Yaw` -73.049204 :`Roll` -32.513389)) "Undefined" "MultiplyWithRoot" null null))))

(fn `ReturnPuzzlePart`
  (returns (PuzzleToPlay :type "UPianoSongData Object Reference"))
  (switch `int` (`self.i_puzzleProgress`)
    (:`Default`
      (return null))
    (:`0`
      (return (`self.da_SongData_1`)))
    (:`1`
      (return (`self.da_SongData_2`)))
    (:`2`
      (return (`self.da_SongData_3`)))
    (:`3`
      (return (`self.da_SongData_4`)))))

(fn `SetupKeyArray`
  (bind _output_get (set `self.KeyComponent` (`|MakeArray` (`self.A0`) (`self.AIS0`) (`self.H0`) (`self.C1`) (`self.CIS1`) (`self.D1`) (`self.DIS1`) (`self.E1`) (`self.F1`) (`self.FIS1`) (`self.G1`) (`self.GIS1`) (`self.A1`) (`self.AIS1`) (`self.H1`) (`self.C2`) (`self.CIS2`) (`self.D2`) (`self.DIS2`) (`self.E2`) (`self.F2`) (`self.FIS2`) (`self.G2`) (`self.GIS2`) (`self.A2`) (`self.AIS2`) (`self.H2`) (`self.C3`) (`self.CIS3`) (`self.D3`) (`self.DIS3`) (`self.E3`) (`self.F3`) (`self.FIS3`) (`self.G3`) (`self.GIS3`) (`self.A3`) (`self.AIS3`) (`self.H3`) (`self.C4`) (`self.CIS4`) (`self.D4`) (`self.DIS4`) (`self.E4`) (`self.F4`) (`self.FIS4`) (`self.G4`) (`self.GIS4`) (`self.A4`) (`self.AIS4`) (`self.H4`) (`self.C5`) (`self.CIS5`) (`self.D5`) (`self.DIS5`) (`self.E5`) (`self.F5`) (`self.FIS5`) (`self.G5`) (`self.GIS5`) (`self.A5`) (`self.AIS5`) (`self.H5`) (`self.C6`) (`self.CIS6`) (`self.D6`) (`self.DIS6`) (`self.E6`) (`self.F6`) (`self.FIS6`) (`self.G6`) (`self.GIS6`) (`self.A6`) (`self.AIS6`) (`self.H6`) (`self.C7`) (`self.CIS7`) (`self.D7`) (`self.DIS7`) (`self.E7`) (`self.F7`) (`self.FIS7`) (`self.G7`) (`self.GIS7`) (`self.A7`) (`self.AIS7`) (`self.H7`) (`self.C8`))))
  (for _array_element _output_get
    (bind _returnvalue (`PrimitiveComponent.CreateDynamicMaterialInstance` _array_element 0 "/Game/HouseEdwards/Assets/LibraryRoom/PianoPuzzle/M_Piano.M_Piano" "None"))
    (bind _output_get_2 (set `self.m_DynMaterial` _returnvalue))
    (`PrimitiveComponent.SetMaterial` _array_element 0 _output_get_2)))

(fn `UserConstructionScript`
  (`self.SetupKeyArray`))