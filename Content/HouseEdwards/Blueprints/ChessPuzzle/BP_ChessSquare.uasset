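; BP_ChessSquare is one board square in the chess puzzle, tracking the piece on it and judging it against that square's solution.
; An overlap detector stores the piece and availability, then asks the parent puzzle actor to check the current round.
; CheckSolution compares piece type, or emptiness, to one of three per-round answers, auto-passing two File values.
; Hover events toggle a highlight plane.
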(event `self.ReceiveBeginPlay`
  ;[0 0.15 0.09358 0.5] General
  (`PrimitiveComponent.SetMaterial` (`self.Plane`) 0 "/Game/HouseEdwards/Blueprints/ChessPuzzle/M_ChessSquare.M_ChessSquare"))

(event `self.PieceDetector.OnComponentBeginOverlap`
  (params (OverlappedComponent :type "PrimitiveComponent Object Reference") (OtherActor :type "Actor Object Reference") (OtherComp :type "PrimitiveComponent Object Reference") (OtherBodyIndex :type Integer) (bFromSweep :type Boolean) (SweepResult :type "HitResult Structure (by ref)"))
  (bind _returnvalue (`self.GetParentActor`))
  ;[0.15 0.01004 0 0.5] Overlap Logic
  ;; Saves CurrentPiece
  (bind _asbp_chess_piece_base (cast `/Game/HouseEdwards/Blueprints/ChessPuzzle/ChessPieces/BP_ChessPiece_Base` OtherActor))
  (set `self.b_isAvailable` false)
  (set `self.a_currentPiece` _asbp_chess_piece_base)
  (bind _asbp_interactable_chess_puzzle (cast `/Game/HouseEdwards/Blueprints/ChessPuzzle/BP_Interactable_ChessPuzzle` _returnvalue)
    (:`then`
      (`/Game/HouseEdwards/Blueprints/ChessPuzzle/BP_Interactable_ChessPuzzle.CheckSolution` _asbp_interactable_chess_puzzle (`/Game/HouseEdwards/Blueprints/ChessPuzzle/BP_Interactable_ChessPuzzle.i_round` _asbp_interactable_chess_puzzle)))
    (:`CastFailed`
      (`KismetSystemLibrary.PrintString` "Cast Failed")
      (`KismetSystemLibrary.PrintString` (`KismetSystemLibrary.GetDisplayName` _returnvalue)))))

(event `self.PieceDetector.OnComponentEndOverlap`
  (params (OverlappedComponent :type "PrimitiveComponent Object Reference") (OtherActor :type "Actor Object Reference") (OtherComp :type "PrimitiveComponent Object Reference") (OtherBodyIndex :type Integer))
  ;[0.15 0.01004 0 0.5] Overlap Logic
  (if (== OtherActor (`self.a_currentPiece`))
    (set `self.a_currentPiece` null)
    (set `self.b_isAvailable` true)))

(event `HoverHighlight`
  ;[0 0.01322 0.15 0.5] Add Hover Glow Effect
  (`SceneComponent.SetVisibility` (`self.Plane`) true false))

(event `HoverUnhighlight`
  ;[0 0.01322 0.15 0.5] Add Hover Glow Effect
  (`SceneComponent.SetVisibility` (`self.Plane`) false false))

(fn `CheckSolution`
  (params (NewParam :type Integer))
  (returns (bool :type Boolean))
  (bind _file (break `/Game/HouseEdwards/Blueprints/ChessPuzzle/Datatypes/STRUCT_SquareIDs` (`self.enum_position`)))
  (if (or (`|EnumEquality` _file "NewEnumerator10") (`|EnumEquality` _file "NewEnumerator8"))
    (return true)
    (else
      (switch `int` NewParam
        (:`1`
          (bind _a_currentpiece (`self.a_currentPiece`)
            (:`then`
              (if (`|EnumEquality` (`/Game/HouseEdwards/Blueprints/ChessPuzzle/ChessPieces/BP_ChessPiece_Base.e_type` _a_currentpiece) (`self.a_solutionR1`))
                (return true)
                (else
                  (return false))))
            (:`else`
              (if (`|EnumEquality` (`self.a_solutionR1`) "NewEnumerator6")
                (return true)
                (else
                  (return false))))))
        (:`2`
          (bind _a_currentpiece_2 (`self.a_currentPiece`)
            (:`then`
              (if (`|EnumEquality` (`/Game/HouseEdwards/Blueprints/ChessPuzzle/ChessPieces/BP_ChessPiece_Base.e_type` _a_currentpiece_2) (`self.a_solutionR2`))
                (return true)
                (else
                  (return false))))
            (:`else`
              (if (`|EnumEquality` (`self.a_solutionR2`) "NewEnumerator6")
                (return true)
                (else
                  (return false))))))
        (:`3`
          (bind _a_currentpiece_3 (`self.a_currentPiece`)
            (:`then`
              (if (`|EnumEquality` (`/Game/HouseEdwards/Blueprints/ChessPuzzle/ChessPieces/BP_ChessPiece_Base.e_type` _a_currentpiece_3) (`self.a_solutionR3`))
                (return true)
                (else
                  (return false))))
            (:`else`
              (if (`|EnumEquality` (`self.a_solutionR3`) "NewEnumerator6")
                (return true)
                (else
                  (return false))))))))))

(fn `UserConstructionScript`)