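; Base actor for chess puzzle pieces, handling hover glow, animated moves and fading.
; Hover sets an emissive color only in a specific player view while the piece is idle.
; A timeline lerps the piece to a destination square with a sine-based height arc and a placement sound; a separate entry moves only black pieces.
; Fading swaps between two dynamic materials and toggles Visibility-channel collision.
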(event `self.ReceiveBeginPlay`
  ;[0 0.15 0.09132 0.5] General
  (bind _returnvalue (`PrimitiveComponent.CreateDynamicMaterialInstance` (`self.StaticMesh`) 0 "/Game/HouseEdwards/Assets/ChessPuzzle/M_Chess_Board_Base_Inst.M_Chess_Board_Base_Inst" "None"))
  (set `self.m_DynMaterialFade` _returnvalue)
  (bind _returnvalue_2 (`PrimitiveComponent.CreateDynamicMaterialInstance` (`self.StaticMesh`) 0 "/Game/HouseEdwards/Assets/ChessPuzzle/M_Chess_Board_Base.M_Chess_Board_Base" "None"))
  (bind _output_get (set `self.m_DynMaterial` _returnvalue_2))
  (`PrimitiveComponent.SetMaterial` (`self.StaticMesh`) 0 _output_get)
  ;; DO NOT TOUCH!!!!!! It's hella ugly, but we do not talk about it
  (`KismetSystemLibrary.Delay` 1.0)
  (`self.K2_SetActorLocation` (`KismetMathLibrary.MakeVector` (.x (`self.K2_GetActorLocation`)) (.y (`self.K2_GetActorLocation`)) (- (.z (`self.K2_GetActorLocation`)) 1.0))))

(event `HoverHighlight`
  ;[0 0.01322 0.15 0.5] Add Hover Glow Effect
  (bind _asbp_player_character (cast `/Game/HouseEdwards/Blueprints/PlayerCharacter/BP_PlayerCharacter` (`GameplayStatics.GetPlayerCharacter` 0)))
  (if (`|EnumEquality` (`/Game/HouseEdwards/Blueprints/PlayerCharacter/BP_PlayerCharacter.enum_currentView` _asbp_player_character) "NewEnumerator1")
    (if (not (`self.b_isMoving`))
      (`MaterialInstanceDynamic.SetVectorParameterValue` (`self.m_DynMaterial`) "EmissiveColor" (struct :`R` 0.36743 :`B` 1.0 :`A` 1.0)))))

(event `HoverUnhighlight`
  ;[0 0.01322 0.15 0.5] Add Hover Glow Effect
  (`MaterialInstanceDynamic.SetVectorParameterValue` :`self` (`self.m_DynMaterial`) :`ParameterName` "EmissiveColor"))

(event `MovePiece`
  (params (destinationSquare :type "/Game/HouseEdwards/Blueprints/ChessPuzzle/BP_ChessSquare Object Reference"))
  ;[0.15 0 0.001498 0.5] Piece Movement
  (set `self.b_isMoving` true)
  (set `self.v_startLocation` (`self.K2_GetActorLocation`))
  (set `self.v_targetLocation` (`self.K2_GetActorLocation` destinationSquare))
  (bind (_direction _height _move) (`Timeline|PieceTimeLine` :!via `PlayFromStart`)
    (:`Update`
      (`self.K2_SetActorLocation` (`KismetMathLibrary.MakeVector` (.x (`KismetMathLibrary.VLerp` (`self.v_startLocation`) (`self.v_targetLocation`) _move)) (.y (`KismetMathLibrary.VLerp` (`self.v_startLocation`) (`self.v_targetLocation`) _move)) (+ (* (`KismetMathLibrary.DegSin` _height) 600.0) (.z (`KismetMathLibrary.VLerp` (`self.v_startLocation`) (`self.v_targetLocation`) _move))))))
    (:`Finished`
      (set `self.b_isMoving` false))
    (:`PlaySound`
      (`GameplayStatics.PlaySound2D` "/Game/HouseEdwards/Assets/Audio/AudioAssets/ChessBoard/SC_PlaceChessPiece.SC_PlaceChessPiece" 1.0 1.0 0.0 null null))))

(event `FadeOut`
  ; Fade Out
  (`PrimitiveComponent.SetMaterial` (`self.StaticMesh`) 0 (`self.m_DynMaterialFade`))
  (bind (_direction _fadeout) (`Timeline|TimelineFadeOut` :!via `PlayFromStart`)
    (:`Update`
      (`MaterialInstanceDynamic.SetScalarParameterValue` (`self.m_DynMaterialFade`) "Opacity" _fadeout)
      (`PrimitiveComponent.SetCollisionResponseToChannel` (`self.StaticMesh`) "ECC_Visibility" "ECR_Ignore"))))

(event `FadeIn`
  ; Fade Out
  (bind (_direction _fadein) (`Timeline|TimelineFadeIn` :!via `PlayFromStart`)
    (:`Update`
      (`MaterialInstanceDynamic.SetScalarParameterValue` (`self.m_DynMaterialFade`) "Opacity" _fadein)
      (`PrimitiveComponent.SetMaterial` (`self.StaticMesh`) 0 (`self.m_DynMaterial`))
      (`PrimitiveComponent.SetCollisionResponseToChannel` (`self.StaticMesh`) "ECC_Visibility" "ECR_Block"))))

(event `MoveBlackPieceToSquare`
  (params (`Destination Square` :type "/Game/HouseEdwards/Blueprints/ChessPuzzle/BP_ChessSquare Object Reference"))
  ;[0 0 0 0.5] Move Black Pieces
  (if (not (`self.b_isWhite`))
    (`self.MovePiece` `Destination Square`)))

(fn `UserConstructionScript`)