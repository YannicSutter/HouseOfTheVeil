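; Interactable chess board puzzle that the player views through a blended camera, moving white pieces with cursor hover and click.
; Each round moves black pieces to hardcoded solution squares, and CheckSolution tests every square before advancing.
; Passing the third round slides the board halves and their pieces apart on a timeline, notifies the game mode and gives the player the brother doll.
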(event `self.ReceiveBeginPlay`
  (bind _a_piecesall (`self.a_piecesAll`))
  ;[0 0.15 0.1045 0.5] General
  ;; Set ChessSquares Array
  (bind _outactors (`GameplayStatics.GetAllActorsOfClass` "/Game/HouseEdwards/Blueprints/ChessPuzzle/BP_ChessSquare.BP_ChessSquare_C"))
  (for _array_element _outactors
    (`KismetArrayLibrary.Array_Add` (`self.a_chessSquares`) _array_element))
  ;; Set ChessPieces Array
  (bind _outactors_2 (`GameplayStatics.GetAllActorsOfClass` "/Game/HouseEdwards/Blueprints/ChessPuzzle/ChessPieces/BP_ChessPiece_Base.BP_ChessPiece_Base_C"))
  (for _array_element_2 _outactors_2
    (if (`/Game/HouseEdwards/Blueprints/ChessPuzzle/ChessPieces/BP_ChessPiece_Base.b_isWhite` _array_element_2)
      (`KismetArrayLibrary.Array_Add` (`self.a_piecesWhite`) _array_element_2)
      (else
        (`KismetArrayLibrary.Array_Add` (`self.a_piecesBlack`) _array_element_2))))
  (`KismetArrayLibrary.Array_Append` _a_piecesall (`self.a_piecesWhite`))
  (`KismetArrayLibrary.Array_Append` _a_piecesall (`self.a_piecesBlack`))
  ;; ChessPuzzle is not always active
  (set `self.b_IsActive` true)
  ;; Sound Settings
  (set `self.sc_InteractSuccess` null)
  (set `self.sc_InteractFail` null)
  (`SceneComponent.SetVisibility` (`self.Indicator White`) false true)
  (`self.SetSolutionsOfPieces`))

(event `self.ReceiveTick`
  (params (DeltaSeconds :type "Float (single-precision)"))
  (bind _a_currentlyhoveredpiece (`self.a_currentlyHoveredPiece`))
  (bind _a_currentlyhoveredsquare (`self.a_currentlyHoveredSquare`))
  (bind (_bblockinghit _binitialoverlap _time _distance _location _impactpoint _normal _impactnormal _physmat _hitactor) (`GameplayStatics.BreakHitResult` (`PlayerController.GetHitResultUnderCursorByChannel` (`GameplayStatics.GetPlayerController` 0) "TraceTypeQuery1" true)))
  ;[0 0.15 0.1045 0.5] General
  (if (`self.b_puzzleSolved`)
    _
    (elif (`self.b_pieceSelectionMode`)
      ;; Chess Pieces
      (bind _asbp_chess_piece_base (cast `/Game/HouseEdwards/Blueprints/ChessPuzzle/ChessPieces/BP_ChessPiece_Base` _hitactor)
        (:`then`
          (if (`KismetArrayLibrary.Array_Contains` (`self.a_piecesWhite`) _asbp_chess_piece_base)
            (`/Engine/EditorBlueprintResources/StandardMacros.IsValid` _a_currentlyhoveredpiece
              (:`Is Valid`
                (`/Game/HouseEdwards/Blueprints/ChessPuzzle/ChessPieces/BP_ChessPiece_Base.HoverUnhighlight` _a_currentlyhoveredpiece))
              (:`Is Not Valid`
                _))
            (bind _output_get (set `self.a_currentlyHoveredPiece` _asbp_chess_piece_base))
            (`/Game/HouseEdwards/Blueprints/ChessPuzzle/ChessPieces/BP_ChessPiece_Base.HoverHighlight` _output_get)
            (else
              (set `self.a_currentlyHoveredPiece` null))))
        (:`CastFailed`
          (`/Engine/EditorBlueprintResources/StandardMacros.IsValid` _a_currentlyhoveredpiece
            (:`Is Valid`
              (`/Game/HouseEdwards/Blueprints/ChessPuzzle/ChessPieces/BP_ChessPiece_Base.HoverUnhighlight` (`self.a_currentlyHoveredPiece`))
              (set `self.a_currentlyHoveredPiece` null)))))
      (else
        ;; Chess Squares
        (bind _asbp_chess_square (cast `/Game/HouseEdwards/Blueprints/ChessPuzzle/BP_ChessSquare` _hitactor)
          (:`then`
            (`/Engine/EditorBlueprintResources/StandardMacros.IsValid` _a_currentlyhoveredsquare
              (:`Is Valid`
                (`/Game/HouseEdwards/Blueprints/ChessPuzzle/BP_ChessSquare.HoverUnhighlight` _a_currentlyhoveredsquare))
              (:`Is Not Valid`
                _))
            (bind _output_get_2 (set `self.a_currentlyHoveredSquare` _asbp_chess_square))
            (`/Game/HouseEdwards/Blueprints/ChessPuzzle/BP_ChessSquare.HoverHighlight` _output_get_2))
          (:`CastFailed`
            (`/Engine/EditorBlueprintResources/StandardMacros.IsValid` _a_currentlyhoveredsquare
              (:`Is Valid`
                (`/Game/HouseEdwards/Blueprints/ChessPuzzle/BP_ChessSquare.HoverUnhighlight` (`self.a_currentlyHoveredSquare`))
                (set `self.a_currentlyHoveredSquare` null)))))))))

(event `self.InteractLogic`
  (bind _returnvalue (`GameplayStatics.GetPlayerController` 0))
  (bind _returnvalue_2 (`GameplayStatics.GetPlayerController` 0))
  (bind _returnvalue_3 (`GameplayStatics.GetPlayerController` 0))
  (bind _returnvalue_4 (pcsubsystem `EnhancedInputLocalPlayerSubsystem` (`GameplayStatics.GetPlayerController` 0)))
  ;[0.15 0.01103 0 0.5] Interact Logic
  (`parent.InteractLogic`)
  (bind _asbp_player_character (cast `/Game/HouseEdwards/Blueprints/PlayerCharacter/BP_PlayerCharacter` (`GameplayStatics.GetPlayerCharacter` 0)))
  (if (not (`self.b_inAnimation`))
    (if (`|EnumEquality` (`/Game/HouseEdwards/Blueprints/PlayerCharacter/BP_PlayerCharacter.enum_currentView` _asbp_player_character) "NewEnumerator1")
      (set `/Game/HouseEdwards/Blueprints/PlayerCharacter/BP_PlayerCharacter.enum_currentView` "NewEnumerator0" _asbp_player_character)
      ;; Handling Controls Input
      (`EnhancedInputSubsystemInterface.AddMappingContext` _returnvalue_4 "/Game/HouseEdwards/Blueprints/PlayerCharacter/Input/IMC_Movement.IMC_Movement" 0 (struct))
      (set `PlayerController.bShowMouseCursor` false _returnvalue_3)
      ;; Set Camera View
      (`PlayerController.SetViewTargetWithBlend` _returnvalue_2 (`GameplayStatics.GetPlayerCharacter` 0) 2.0 "VTBlend_EaseInOut" 1.5 false)
      (`SceneComponent.SetVisibility` (`self.Indicator White`) false true)
      (`WidgetBlueprintLibrary.SetInputMode_GameOnly` _returnvalue)
      (`Widget.RemoveFromParent` (`self.wbp_exitUI`))
      (else
        (set `/Game/HouseEdwards/Blueprints/PlayerCharacter/BP_PlayerCharacter.enum_currentView` "NewEnumerator1" _asbp_player_character)
        (`EnhancedInputSubsystemInterface.RemoveMappingContext` _returnvalue_4 "/Game/HouseEdwards/Blueprints/PlayerCharacter/Input/IMC_Movement.IMC_Movement" (struct))
        (set `PlayerController.bShowMouseCursor` true _returnvalue_3)
        (`PlayerController.SetViewTargetWithBlend` _returnvalue_2 self 2.0 "VTBlend_EaseInOut" 2.0 false)
        (`SceneComponent.SetVisibility` (`self.Indicator White`) true true)
        (`WidgetBlueprintLibrary.SetInputMode_GameAndUIEx` _returnvalue null)
        (bind _returnvalue_5 (`|CreateWidget` "/Game/HouseEdwards/Blueprints/ChessPuzzle/WBP_exitUI.WBP_exitUI_C" (`GameplayStatics.GetPlayerController` 0)))
        (bind _output_get (set `self.wbp_exitUI` _returnvalue_5))
        (`UserWidget.AddToViewport` _output_get 0)
        (if (`self.b_firstInteraction`)
          (`KismetSystemLibrary.Delay` 2.5)
          (set `self.b_firstInteraction` false)
          (`self.MoveBlackPieces` (`self.i_round`)))))))

(event `HandleClick`
  ;[0.15 0.01103 0 0.5] Interact Logic
  (if (or (`self.b_puzzleSolved`) (`self.b_inAnimation`))
    _
    (elif (`self.b_pieceSelectionMode`)
      (if (!= (`self.a_currentlyHoveredPiece`) null)
        (set `self.b_pieceSelectionMode` false)
        (bind _output_get (set `self.a_selectedPiece` (`self.a_currentlyHoveredPiece`)))
        (`/Game/HouseEdwards/Blueprints/ChessPuzzle/ChessPieces/BP_ChessPiece_Base.HoverUnhighlight` _output_get)
        (for _array_element (`self.a_piecesAll`)
          (`/Game/HouseEdwards/Blueprints/ChessPuzzle/ChessPieces/BP_ChessPiece_Base.FadeOut` _array_element)))
      (else
        (bind _a_currentlyhoveredsquare (`self.a_currentlyHoveredSquare`)
          (:`then`
            (if (!= (`/Game/HouseEdwards/Blueprints/ChessPuzzle/BP_ChessSquare.a_currentPiece` _a_currentlyhoveredsquare) (`self.a_selectedPiece`))
              (if (`/Game/HouseEdwards/Blueprints/ChessPuzzle/BP_ChessSquare.b_isAvailable` _a_currentlyhoveredsquare)
                (bind _output_get_2 (set `self.a_selectedSquare` (`self.a_currentlyHoveredSquare`)))
                (`/Game/HouseEdwards/Blueprints/ChessPuzzle/BP_ChessSquare.HoverUnhighlight` _output_get_2)
                (`/Game/HouseEdwards/Blueprints/ChessPuzzle/ChessPieces/BP_ChessPiece_Base.MovePiece` (`self.a_selectedPiece`) _output_get_2)
                (for _array_element_2 (`self.a_piecesAll`) :!label _label
                  (`/Game/HouseEdwards/Blueprints/ChessPuzzle/ChessPieces/BP_ChessPiece_Base.FadeIn` _array_element_2))
                (set `self.b_pieceSelectionMode` true)
                (set `self.a_selectedPiece` null)
                (set `self.a_selectedSquare` null)
                (set `self.b_inAnimation` true)
                (`KismetSystemLibrary.Delay` 2.0)
                (set `self.b_inAnimation` false))
              (else
                (`/Game/HouseEdwards/Blueprints/ChessPuzzle/BP_ChessSquare.HoverUnhighlight` _a_currentlyhoveredsquare)
                (goto _label))))
          (:`else`))))))

(event `MoveBlackPieces`
  (params (Round :type Integer))
  ;[0.005208 0.005208 0.005208 0.5] Move Black Pieces
  (for _array_element (`self.a_piecesBlack`)
    (switch `int` Round
      (:`1`
        (for _array_element_2 (`self.a_chessSquares`)
          (bind (_file _rank) (break `/Game/HouseEdwards/Blueprints/ChessPuzzle/Datatypes/STRUCT_SquareIDs` (`/Game/HouseEdwards/Blueprints/ChessPuzzle/BP_ChessSquare.enum_position` _array_element_2)))
          (bind (_file_2 _rank_2) (break `/Game/HouseEdwards/Blueprints/ChessPuzzle/Datatypes/STRUCT_SquareIDs` (`/Game/HouseEdwards/Blueprints/ChessPuzzle/ChessPieces/BP_ChessPiece_Base.a_solution1` _array_element)))
          (if (and (`|EnumEquality` _file _file_2) (`|EnumEquality` _rank _rank_2))
            (`/Game/HouseEdwards/Blueprints/ChessPuzzle/ChessPieces/BP_ChessPiece_Base.MoveBlackPieceToSquare` _array_element _array_element_2))))
      (:`2`
        (for _array_element_3 (`self.a_chessSquares`)
          (bind (_file_3 _rank_3) (break `/Game/HouseEdwards/Blueprints/ChessPuzzle/Datatypes/STRUCT_SquareIDs` (`/Game/HouseEdwards/Blueprints/ChessPuzzle/BP_ChessSquare.enum_position` _array_element_3)))
          (bind (_file_4 _rank_4) (break `/Game/HouseEdwards/Blueprints/ChessPuzzle/Datatypes/STRUCT_SquareIDs` (`/Game/HouseEdwards/Blueprints/ChessPuzzle/ChessPieces/BP_ChessPiece_Base.a_solution2` _array_element)))
          (if (and (`|EnumEquality` _file_3 _file_4) (`|EnumEquality` _rank_3 _rank_4))
            (`/Game/HouseEdwards/Blueprints/ChessPuzzle/ChessPieces/BP_ChessPiece_Base.MoveBlackPieceToSquare` _array_element _array_element_3))))
      (:`3`
        (for _array_element_4 (`self.a_chessSquares`)
          (bind (_file_5 _rank_5) (break `/Game/HouseEdwards/Blueprints/ChessPuzzle/Datatypes/STRUCT_SquareIDs` (`/Game/HouseEdwards/Blueprints/ChessPuzzle/BP_ChessSquare.enum_position` _array_element_4)))
          (bind (_file_6 _rank_6) (break `/Game/HouseEdwards/Blueprints/ChessPuzzle/Datatypes/STRUCT_SquareIDs` (`/Game/HouseEdwards/Blueprints/ChessPuzzle/ChessPieces/BP_ChessPiece_Base.a_solution3` _array_element)))
          (if (and (`|EnumEquality` _file_5 _file_6) (`|EnumEquality` _rank_5 _rank_6))
            (`/Game/HouseEdwards/Blueprints/ChessPuzzle/ChessPieces/BP_ChessPiece_Base.MoveBlackPieceToSquare` _array_element _array_element_4))))))
  (set `self.b_inAnimation` true)
  (`KismetSystemLibrary.Delay` 2.0)
  (set `self.b_inAnimation` false))

(event `OpenBoard`
  ; Open Board
  (for _array_element (`self.a_chessSquares`)
    (bind _a_currentpiece (`/Game/HouseEdwards/Blueprints/ChessPuzzle/BP_ChessSquare.a_currentPiece` _array_element))
    (if (and (`/Game/HouseEdwards/Blueprints/ChessPuzzle/BP_ChessSquare.b_isOnBoard` _array_element) (`KismetSystemLibrary.IsValid` _a_currentpiece))
      (if (>= (.y (`KismetMathLibrary.InverseTransformLocation` (`self.GetTransform`) (`self.K2_GetActorLocation` _a_currentpiece))) 0.0)
        (`KismetArrayLibrary.Array_Add` (`self.LeftSideActors`) _a_currentpiece)
        (else
          (`KismetArrayLibrary.Array_Add` (`self.RightSideActors`) _a_currentpiece)))))
  (bind (_direction _openboardleftside _openboardrightside) (`Timeline|OpenBoardBothSides` :!via `PlayFromStart`)
    (:`Update`
      ;; Board Sides
      (`SceneComponent.K2_AddLocalOffset` (`self.Side1`) (`KismetMathLibrary.MakeVector` _openboardrightside) false false)
      (`SceneComponent.K2_AddLocalOffset` (`self.Side2`) (`KismetMathLibrary.MakeVector` _openboardleftside) false false)
      (for _array_element_2 (`self.LeftSideActors`)
        (`self.K2_AddActorLocalOffset` _array_element_2 (`KismetMathLibrary.MakeVector` 0.0 _openboardleftside) false false))
      (for _array_element_3 (`self.RightSideActors`)
        (`self.K2_AddActorLocalOffset` _array_element_3 (`KismetMathLibrary.MakeVector` 0.0 _openboardrightside) false false)))
    (:`Finished`
      (`Widget.RemoveFromParent` (`self.wbp_exitUI`))
      (bind _asgm_base (cast `/Game/HouseEdwards/Blueprints/Gamemodes/GM_Base` (`GameplayStatics.GetGameMode`)))
      (`/Game/HouseEdwards/Blueprints/Gamemodes/GM_Base.SolvedChessPuzzle` _asgm_base)
      (set `self.b_puzzleSolved` true)
      (bind _asbp_player_character (cast `/Game/HouseEdwards/Blueprints/PlayerCharacter/BP_PlayerCharacter` (`GameplayStatics.GetPlayerCharacter` 0)))
      (bind _asbp_interactable_doll_brother (cast `/Game/HouseEdwards/Blueprints/Interactables/BP_Interactable_Doll_Brother` (`ChildActorComponent.ChildActor` (`self.Doll`))))
      (`PlayerController.SetViewTargetWithBlend` (`GameplayStatics.GetPlayerController` 0) (`GameplayStatics.GetPlayerCharacter` 0) 2.0 "VTBlend_EaseInOut" 1.5 true)
      (`WidgetBlueprintLibrary.SetInputMode_GameOnly` (`GameplayStatics.GetPlayerController` 0))
      (set `/Game/HouseEdwards/Blueprints/PlayerCharacter/BP_PlayerCharacter.enum_currentView` "NewEnumerator0" _asbp_player_character)
      (`EnhancedInputSubsystemInterface.AddMappingContext` (pcsubsystem `EnhancedInputLocalPlayerSubsystem` (`GameplayStatics.GetPlayerController` 0)) "/Game/HouseEdwards/Blueprints/PlayerCharacter/Input/IMC_Movement.IMC_Movement" 0 (struct))
      (set `PlayerController.bShowMouseCursor` false (`GameplayStatics.GetPlayerController` 0))
      (`KismetSystemLibrary.Delay` 2.0)
      (`StaticMeshComponent.SetStaticMesh` (`/Game/HouseEdwards/Blueprints/PlayerCharacter/BP_PlayerCharacter.Doll` _asbp_player_character) (`StaticMeshComponent.StaticMesh` (`/Game/HouseEdwards/Blueprints/Interactables/BP_Interactable_Doll.Static Mesh` _asbp_interactable_doll_brother)))
      (set `/Game/HouseEdwards/Blueprints/PlayerCharacter/BP_PlayerCharacter.b_hasDoll` true _asbp_player_character)
      (`self.K2_DestroyActor` (`ChildActorComponent.ChildActor` (`self.Doll`))))
    (:`Audio`
      (`GameplayStatics.PlaySoundAtLocation` "/Game/HouseEdwards/Assets/Audio/AudioAssets/ChessBoard/SC_OpenChessBoard.SC_OpenChessBoard" (`self.K2_GetActorLocation`) (struct) 1.0 1.0 0.0 null null null null))))

(event `SetSolutionsOfPieces`
  ;[0 0.15 0.1421 0.5] Set Solutions
  (`self.SetupSolution` (`self.BP_PawnBlack`) (make `/Game/HouseEdwards/Blueprints/ChessPuzzle/Datatypes/STRUCT_SquareIDs` "NewEnumerator9" "NewEnumerator16") (make `/Game/HouseEdwards/Blueprints/ChessPuzzle/Datatypes/STRUCT_SquareIDs` "NewEnumerator8") (make `/Game/HouseEdwards/Blueprints/ChessPuzzle/Datatypes/STRUCT_SquareIDs` "NewEnumerator9" "NewEnumerator16"))
  (`self.SetupSolution` (`self.BP_PawnBlack1`) (make `/Game/HouseEdwards/Blueprints/ChessPuzzle/Datatypes/STRUCT_SquareIDs` "NewEnumerator9" "NewEnumerator16") (make `/Game/HouseEdwards/Blueprints/ChessPuzzle/Datatypes/STRUCT_SquareIDs` "NewEnumerator9" "NewEnumerator16") (make `/Game/HouseEdwards/Blueprints/ChessPuzzle/Datatypes/STRUCT_SquareIDs` "NewEnumerator9" "NewEnumerator16"))
  (`self.SetupSolution` (`self.BP_PawnBlack2`) (make `/Game/HouseEdwards/Blueprints/ChessPuzzle/Datatypes/STRUCT_SquareIDs` "NewEnumerator9" "NewEnumerator16") (make `/Game/HouseEdwards/Blueprints/ChessPuzzle/Datatypes/STRUCT_SquareIDs` "NewEnumerator8" "NewEnumerator1") (make `/Game/HouseEdwards/Blueprints/ChessPuzzle/Datatypes/STRUCT_SquareIDs` "NewEnumerator9" "NewEnumerator16"))
  (`self.SetupSolution` (`self.BP_PawnBlack3`) (make `/Game/HouseEdwards/Blueprints/ChessPuzzle/Datatypes/STRUCT_SquareIDs` "NewEnumerator9" "NewEnumerator16") (make `/Game/HouseEdwards/Blueprints/ChessPuzzle/Datatypes/STRUCT_SquareIDs` "NewEnumerator9" "NewEnumerator16") (make `/Game/HouseEdwards/Blueprints/ChessPuzzle/Datatypes/STRUCT_SquareIDs` "NewEnumerator9" "NewEnumerator16"))
  (`self.SetupSolution` (`self.BP_PawnBlack4`) (make `/Game/HouseEdwards/Blueprints/ChessPuzzle/Datatypes/STRUCT_SquareIDs` "NewEnumerator9" "NewEnumerator16") (make `/Game/HouseEdwards/Blueprints/ChessPuzzle/Datatypes/STRUCT_SquareIDs` "NewEnumerator9" "NewEnumerator16") (make `/Game/HouseEdwards/Blueprints/ChessPuzzle/Datatypes/STRUCT_SquareIDs` "NewEnumerator9" "NewEnumerator16"))
  (`self.SetupSolution` (`self.BP_PawnBlack5`) (make `/Game/HouseEdwards/Blueprints/ChessPuzzle/Datatypes/STRUCT_SquareIDs` "NewEnumerator3" "NewEnumerator5") (make `/Game/HouseEdwards/Blueprints/ChessPuzzle/Datatypes/STRUCT_SquareIDs` "NewEnumerator8" "NewEnumerator2") (make `/Game/HouseEdwards/Blueprints/ChessPuzzle/Datatypes/STRUCT_SquareIDs` "NewEnumerator9" "NewEnumerator16"))
  (`self.SetupSolution` (`self.BP_PawnBlack6`) (make `/Game/HouseEdwards/Blueprints/ChessPuzzle/Datatypes/STRUCT_SquareIDs` "NewEnumerator4" "NewEnumerator4") (make `/Game/HouseEdwards/Blueprints/ChessPuzzle/Datatypes/STRUCT_SquareIDs` "NewEnumerator9" "NewEnumerator16") (make `/Game/HouseEdwards/Blueprints/ChessPuzzle/Datatypes/STRUCT_SquareIDs` "NewEnumerator9" "NewEnumerator16"))
  (`self.SetupSolution` (`self.BP_PawnBlack7`) (make `/Game/HouseEdwards/Blueprints/ChessPuzzle/Datatypes/STRUCT_SquareIDs` "NewEnumerator9" "NewEnumerator16") (make `/Game/HouseEdwards/Blueprints/ChessPuzzle/Datatypes/STRUCT_SquareIDs` "NewEnumerator9" "NewEnumerator16") (make `/Game/HouseEdwards/Blueprints/ChessPuzzle/Datatypes/STRUCT_SquareIDs` "NewEnumerator9" "NewEnumerator16"))
  (`self.SetupSolution` (`self.BP_RookBlack`) (make `/Game/HouseEdwards/Blueprints/ChessPuzzle/Datatypes/STRUCT_SquareIDs` "NewEnumerator9" "NewEnumerator16") (make `/Game/HouseEdwards/Blueprints/ChessPuzzle/Datatypes/STRUCT_SquareIDs` "NewEnumerator3" "NewEnumerator7") (make `/Game/HouseEdwards/Blueprints/ChessPuzzle/Datatypes/STRUCT_SquareIDs` "NewEnumerator8" "NewEnumerator4"))
  (`self.SetupSolution` (`self.BP_RookBlack1`) (make `/Game/HouseEdwards/Blueprints/ChessPuzzle/Datatypes/STRUCT_SquareIDs` "NewEnumerator9" "NewEnumerator16") (make `/Game/HouseEdwards/Blueprints/ChessPuzzle/Datatypes/STRUCT_SquareIDs` "NewEnumerator9" "NewEnumerator16") (make `/Game/HouseEdwards/Blueprints/ChessPuzzle/Datatypes/STRUCT_SquareIDs` "NewEnumerator9" "NewEnumerator16"))
  (`self.SetupSolution` (`self.BP_KnightBlack`) (make `/Game/HouseEdwards/Blueprints/ChessPuzzle/Datatypes/STRUCT_SquareIDs` "NewEnumerator9" "NewEnumerator16") (make `/Game/HouseEdwards/Blueprints/ChessPuzzle/Datatypes/STRUCT_SquareIDs` "NewEnumerator5" "NewEnumerator5") (make `/Game/HouseEdwards/Blueprints/ChessPuzzle/Datatypes/STRUCT_SquareIDs` "NewEnumerator8" "NewEnumerator5"))
  (`self.SetupSolution` (`self.BP_KnightBlack1`) (make `/Game/HouseEdwards/Blueprints/ChessPuzzle/Datatypes/STRUCT_SquareIDs` "NewEnumerator9" "NewEnumerator16") (make `/Game/HouseEdwards/Blueprints/ChessPuzzle/Datatypes/STRUCT_SquareIDs` "NewEnumerator3" "NewEnumerator6") (make `/Game/HouseEdwards/Blueprints/ChessPuzzle/Datatypes/STRUCT_SquareIDs` "NewEnumerator1" "NewEnumerator7"))
  (`self.SetupSolution` (`self.BP_BishopBlack`) (make `/Game/HouseEdwards/Blueprints/ChessPuzzle/Datatypes/STRUCT_SquareIDs` "NewEnumerator9" "NewEnumerator16") (make `/Game/HouseEdwards/Blueprints/ChessPuzzle/Datatypes/STRUCT_SquareIDs` "NewEnumerator9" "NewEnumerator16") (make `/Game/HouseEdwards/Blueprints/ChessPuzzle/Datatypes/STRUCT_SquareIDs` "NewEnumerator9" "NewEnumerator16"))
  (`self.SetupSolution` (`self.BP_BishopBlack1`) (make `/Game/HouseEdwards/Blueprints/ChessPuzzle/Datatypes/STRUCT_SquareIDs` "NewEnumerator9" "NewEnumerator16") (make `/Game/HouseEdwards/Blueprints/ChessPuzzle/Datatypes/STRUCT_SquareIDs` "NewEnumerator8" "NewEnumerator3") (make `/Game/HouseEdwards/Blueprints/ChessPuzzle/Datatypes/STRUCT_SquareIDs` "NewEnumerator9" "NewEnumerator16"))
  (`self.SetupSolution` (`self.BP_QueenBlack`) (make `/Game/HouseEdwards/Blueprints/ChessPuzzle/Datatypes/STRUCT_SquareIDs` "NewEnumerator9" "NewEnumerator16") (make `/Game/HouseEdwards/Blueprints/ChessPuzzle/Datatypes/STRUCT_SquareIDs` "NewEnumerator4" "NewEnumerator6") (make `/Game/HouseEdwards/Blueprints/ChessPuzzle/Datatypes/STRUCT_SquareIDs` "NewEnumerator4" "NewEnumerator5"))
  (`self.SetupSolution` (`self.BP_KingBlack`) (make `/Game/HouseEdwards/Blueprints/ChessPuzzle/Datatypes/STRUCT_SquareIDs` "NewEnumerator9" "NewEnumerator16") (make `/Game/HouseEdwards/Blueprints/ChessPuzzle/Datatypes/STRUCT_SquareIDs` "NewEnumerator9" "NewEnumerator16") (make `/Game/HouseEdwards/Blueprints/ChessPuzzle/Datatypes/STRUCT_SquareIDs` "NewEnumerator9" "NewEnumerator16")))

(fn `CheckSolution`
  (params (Round :type Integer))
  (returns (Solution :type Boolean))
  (for _array_element (`self.a_chessSquares`)
    (bind _bool (`/Game/HouseEdwards/Blueprints/ChessPuzzle/BP_ChessSquare.CheckSolution` _array_element Round))
    (if (not _bool)
      (return false)))
  (if (>= Round 3)
    (`self.OpenBoard`)
    (return true)
    (else
      (bind _output_get (set `self.i_round` (+ Round 1)))
      (`/Game/HouseEdwards/Blueprints/ChessPuzzle/WBP_exitUI.PlaySuccessText` (`self.wbp_exitUI`))
      (`self.MoveBlackPieces` _output_get)
      (return true))))

(fn `SetupSolution`
  (params (ChessPiece :type "ChildActorComponent Object Reference") (a_solution1 :type "/Game/HouseEdwards/Blueprints/ChessPuzzle/Datatypes/STRUCT_SquareIDs Structure") (a_solution2 :type "/Game/HouseEdwards/Blueprints/ChessPuzzle/Datatypes/STRUCT_SquareIDs Structure") (a_solution3 :type "/Game/HouseEdwards/Blueprints/ChessPuzzle/Datatypes/STRUCT_SquareIDs Structure"))
  (bind _asbp_chess_piece_base (cast `/Game/HouseEdwards/Blueprints/ChessPuzzle/ChessPieces/BP_ChessPiece_Base` (`ChildActorComponent.ChildActor` ChessPiece)))
  (set `/Game/HouseEdwards/Blueprints/ChessPuzzle/ChessPieces/BP_ChessPiece_Base.a_solution1` a_solution1 _asbp_chess_piece_base)
  (set `/Game/HouseEdwards/Blueprints/ChessPuzzle/ChessPieces/BP_ChessPiece_Base.a_solution2` a_solution2 _asbp_chess_piece_base)
  (set `/Game/HouseEdwards/Blueprints/ChessPuzzle/ChessPieces/BP_ChessPiece_Base.a_solution3` a_solution3 _asbp_chess_piece_base))

(fn `UserConstructionScript`)