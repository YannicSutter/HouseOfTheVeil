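; House ambience actor that uses a timeline as a cooldown for playing an environment sound at its location.
; While the player is outside its box trigger, Tick restarts the timeline whenever it stops, through its component reference.
; The timeline's Cooldown event plays the sound.
; BeginPlay sets a random timeline position, which PlayFromStart resets, so the interval is not actually randomized.
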(event `self.ReceiveBeginPlay`
  (`TimelineComponent.SetNewTime` (`self.ti_enviroment_SoundEffect`) (`KismetMathLibrary.RandomFloatInRange` 15.0 40.0)))

(event `self.ReceiveTick`
  (params (DeltaSeconds :type "Float (single-precision)"))
  (bind _ti_enviroment_soundeffect (`self.ti_enviroment_SoundEffect`))
  (if (!= (`self.b_playerIsInRange`) true)
    (if (not (`TimelineComponent.IsPlaying` _ti_enviroment_soundeffect))
      (`TimelineComponent.PlayFromStart` _ti_enviroment_soundeffect))))

(event `self.BoxTrigger.OnComponentEndOverlap`
  (params (OverlappedComponent :type "PrimitiveComponent Object Reference") (OtherActor :type "Actor Object Reference") (OtherComp :type "PrimitiveComponent Object Reference") (OtherBodyIndex :type Integer))
  (cast `/Game/HouseEdwards/Blueprints/PlayerCharacter/BP_PlayerCharacter` OtherActor)
  (set `self.b_playerIsInRange` false))

(event `self.BoxTrigger.OnComponentBeginOverlap`
  (params (OverlappedComponent :type "PrimitiveComponent Object Reference") (OtherActor :type "Actor Object Reference") (OtherComp :type "PrimitiveComponent Object Reference") (OtherBodyIndex :type Integer) (bFromSweep :type Boolean) (SweepResult :type "HitResult Structure (by ref)"))
  (cast `/Game/HouseEdwards/Blueprints/PlayerCharacter/BP_PlayerCharacter` OtherActor)
  (set `self.b_playerIsInRange` true))

(fn `UserConstructionScript`)