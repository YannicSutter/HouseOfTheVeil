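; BP_Interactable_Doll is an interactable pickup that gives the player a doll.
; On BeginPlay it sets itself active and clears the inherited interact success and fail sounds.
; When interacted with, it runs the parent logic, copies its static mesh onto the player character's Doll component, sets the player's has-doll flag and destroys itself.
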(event `self.ReceiveBeginPlay`
  ;[0 0.1615 0.1313 0.5] General
  (`parent.ReceiveBeginPlay`)
  ;; Dolls have to be activated manually
  (set `self.b_IsActive` true)
  ;; Sound Settings
  (set `self.sc_InteractSuccess` null)
  (set `self.sc_InteractFail` null))

(event `self.ReceiveTick`
  (params (DeltaSeconds :type "Float (single-precision)"))
  ;[0 0.1615 0.1313 0.5] General
  (`parent.ReceiveTick` DeltaSeconds))

(event `self.InteractLogic`
  ;[0.15 0.01341 0 0.5] Interact Logic
  (`parent.InteractLogic`)
  (bind _asbp_player_character (cast `/Game/HouseEdwards/Blueprints/PlayerCharacter/BP_PlayerCharacter` (`GameplayStatics.GetPlayerCharacter` 0)))
  (`StaticMeshComponent.SetStaticMesh` (`/Game/HouseEdwards/Blueprints/PlayerCharacter/BP_PlayerCharacter.Doll` _asbp_player_character) (`StaticMeshComponent.StaticMesh` (`self.Static Mesh`)))
  (set `/Game/HouseEdwards/Blueprints/PlayerCharacter/BP_PlayerCharacter.b_hasDoll` true _asbp_player_character)
  (`self.K2_DestroyActor`))

(fn `UserConstructionScript`
  (`parent.UserConstructionScript`))