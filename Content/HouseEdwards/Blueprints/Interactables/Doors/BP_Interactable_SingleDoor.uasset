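; BP_Interactable_SingleDoor is an interactable single door that stays locked until it is activated.
; InteractLogic plays a locked sound while inactive; when active, it calls DoorFlipFlop, which alternates between opening and closing with matching sounds.
; A timeline rotates the door mesh 90 degrees in yaw, and an animation flag blocks re-triggering until it finishes.
; BeginPlay clears the parent's success and fail sounds and starts the door inactive.
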(event `self.ReceiveBeginPlay`
  ;[0 0.1615 0.1313 0.5] General
  (`parent.ReceiveBeginPlay`)
  ;; Doors have to be activated manually
  (set `self.b_IsActive` false)
  ;; Sound Settings
  (set `self.sc_InteractSuccess` null)
  (set `self.sc_InteractFail` null))

(event `self.InteractLogic`
  ;[0.15 0.01341 0 0.5] Interact Logic
  (`parent.InteractLogic`)
  (if (`self.b_IsActive`)
    (`self.DoorFlipFlop`)
    (else
      (`GameplayStatics.PlaySoundAtLocation` "/Game/HouseEdwards/Assets/Audio/AudioAssets/Door/SC_DoorLocked_Cue.SC_DoorLocked_Cue" (`self.K2_GetActorLocation`) (struct) 1.0 1.0 0.0 null null null null))))

(event `DoorFlipFlop`
  ;[0 0.04553 0.15 0.5] Open / Close Door
  (if (not (`self.b_isInAnimation`))
    (set `self.b_isInAnimation` true)
    (`/Engine/EditorBlueprintResources/StandardMacros.FlipFlop`
      (:`A`
        ;; Audio for opening/closing the Door
        (`GameplayStatics.PlaySoundAtLocation` "/Game/HouseEdwards/Assets/Audio/AudioAssets/Door/SC_DoorOpen.SC_DoorOpen" (`self.K2_GetActorLocation`) (struct) 1.0 1.0 0.0 null null null null)
        (bind (_direction _open) (`Timeline|Open` :!via `PlayFromStart` :!label _label)
          (:`Update`
            (`SceneComponent.K2_SetRelativeRotation` (`self.Door`) (`KismetMathLibrary.MakeRotator` 0.0 0.0 (`KismetMathLibrary.Lerp` 0.0 -90.0 _open)) false false))
          (:`Finished`
            (set `self.b_isInAnimation` false))))
      (:`B`
        (`GameplayStatics.PlaySoundAtLocation` "/Game/HouseEdwards/Assets/Audio/AudioAssets/Door/SC_DoorClose.SC_DoorClose" (`self.K2_GetActorLocation`) (struct) 1.0 1.0 0.0 null null null null)
        (goto _label :!via `ReverseFromEnd`)))))

(fn `UserConstructionScript`
  (`parent.UserConstructionScript`))