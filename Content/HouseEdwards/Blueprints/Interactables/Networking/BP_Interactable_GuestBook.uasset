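; Interactable guest book that starts inactive and toggles an on-screen guestbook widget when the player interacts with it.
; Each interaction runs the parent logic, plays a sound, then uses the player character's current view enum as the open/closed state.
; Opening removes the movement mapping context, creates WBP_Guestbook and shows the cursor in Game and UI input.
; Closing restores movement and game-only input and removes the widget.
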(event `self.ReceiveBeginPlay`
  ;[0 0.15 0.0501 0.5] General
  (`parent.ReceiveBeginPlay`)
  ;; The guestbook is not always active
  (set `self.b_IsActive` false))

(event `self.InteractLogic`
  (bind _returnvalue (`GameplayStatics.GetPlayerController` 0))
  (bind _returnvalue_2 (`GameplayStatics.GetPlayerController` 0))
  (bind _returnvalue_3 (pcsubsystem `EnhancedInputLocalPlayerSubsystem` (`GameplayStatics.GetPlayerController` 0)))
  ;[0.15 0.001181 0 0.5] Interact Logic
  (`parent.InteractLogic`)
  (bind _asbp_player_character (cast `/Game/HouseEdwards/Blueprints/PlayerCharacter/BP_PlayerCharacter` (`GameplayStatics.GetPlayerCharacter` 0)))
  (`GameplayStatics.PlaySound2D` "/Game/HouseEdwards/Assets/Audio/AudioAssets/Paper/SC_GuestBook.SC_GuestBook" 1.0 1.0 0.0 null null)
  (if (`|EnumEquality` (`/Game/HouseEdwards/Blueprints/PlayerCharacter/BP_PlayerCharacter.enum_currentView` _asbp_player_character) "NewEnumerator6")
    (set `/Game/HouseEdwards/Blueprints/PlayerCharacter/BP_PlayerCharacter.enum_currentView` "NewEnumerator0" _asbp_player_character)
    (`EnhancedInputSubsystemInterface.AddMappingContext` _returnvalue_3 "/Game/HouseEdwards/Blueprints/PlayerCharacter/Input/IMC_Movement.IMC_Movement" 0 (struct))
    (bind _wbp_guestbook (`self.wbp_Guestbook`)
      (:`then`
        (`Widget.RemoveFromParent` _wbp_guestbook)
        (set `self.wbp_Guestbook` null)
        (set `PlayerController.bShowMouseCursor` false _returnvalue_2)
        (`WidgetBlueprintLibrary.SetInputMode_GameOnly` _returnvalue_2))
      (:`else`))
    (else
      (set `/Game/HouseEdwards/Blueprints/PlayerCharacter/BP_PlayerCharacter.enum_currentView` "NewEnumerator6" _asbp_player_character)
      (`EnhancedInputSubsystemInterface.RemoveMappingContext` _returnvalue_3 "/Game/HouseEdwards/Blueprints/PlayerCharacter/Input/IMC_Movement.IMC_Movement" (struct))
      (bind _returnvalue_4 (`|CreateWidget` "/Game/HouseEdwards/Blueprints/Interactables/Networking/WBP_Guestbook.WBP_Guestbook_C" (`GameplayStatics.GetPlayerController` 0)))
      (`UserWidget.AddToViewport` _returnvalue_4 0)
      (bind _output_get (set `self.wbp_Guestbook` _returnvalue_4))
      (set `PlayerController.bShowMouseCursor` true _returnvalue)
      (`WidgetBlueprintLibrary.SetInputMode_GameAndUIEx` _returnvalue _output_get))))

(fn `UserConstructionScript`
  (`parent.UserConstructionScript`))