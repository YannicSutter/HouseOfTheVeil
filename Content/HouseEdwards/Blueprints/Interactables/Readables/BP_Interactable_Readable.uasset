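; BP_Interactable_Readable is an always-active interactable paper that the player can read up close.
; Its texture feeds a dynamic material on the Plane, set in the Construction Script and at BeginPlay.
; Interacting toggles the player's view state, removing or restoring the movement mapping context.
; The same toggle creates or removes a WBP_ReadableViewer widget showing that texture, with a paper-handling sound.
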(event `self.ReceiveBeginPlay`
  ;[0 0 0 0.5] General
  (`parent.ReceiveBeginPlay`)
  ;; Readables are always active
  (set `self.b_IsActive` true)
  (bind _returnvalue (`PrimitiveComponent.CreateDynamicMaterialInstance` (`self.Plane`) 0 "/Game/HouseEdwards/Blueprints/Interactables/Readables/M_Readable.M_Readable" "None"))
  (`MaterialInstanceDynamic.SetTextureParameterValue` _returnvalue "Texture" (`self.t_Texture`)))

(event `self.InteractLogic`
  (bind _returnvalue (pcsubsystem `EnhancedInputLocalPlayerSubsystem` (`GameplayStatics.GetPlayerController` 0)))
  ;[0.3038 0.01248 0 0.5] Interact Logic
  (`parent.InteractLogic`)
  (bind _asbp_player_character (cast `/Game/HouseEdwards/Blueprints/PlayerCharacter/BP_PlayerCharacter` (`GameplayStatics.GetPlayerCharacter` 0)))
  (if (`|EnumEquality` (`/Game/HouseEdwards/Blueprints/PlayerCharacter/BP_PlayerCharacter.enum_currentView` _asbp_player_character) "NewEnumerator6")
    (set `/Game/HouseEdwards/Blueprints/PlayerCharacter/BP_PlayerCharacter.enum_currentView` "NewEnumerator0" _asbp_player_character)
    ;; Handling Controls Input
    (`EnhancedInputSubsystemInterface.AddMappingContext` _returnvalue "/Game/HouseEdwards/Blueprints/PlayerCharacter/Input/IMC_Movement.IMC_Movement" 0 (struct))
    (bind _w_widget (`self.w_Widget`)
      (:`then`
        (`Widget.RemoveFromParent` _w_widget)
        (set `self.w_Widget` _w_widget)
        (`GameplayStatics.PlaySound2D` "/Game/HouseEdwards/Assets/Audio/AudioAssets/Paper/SC_HandlePaper.SC_HandlePaper" 1.0 1.0 0.0 null null))
      (:`else`))
    (else
      (set `/Game/HouseEdwards/Blueprints/PlayerCharacter/BP_PlayerCharacter.enum_currentView` "NewEnumerator6" _asbp_player_character)
      (`EnhancedInputSubsystemInterface.RemoveMappingContext` _returnvalue "/Game/HouseEdwards/Blueprints/PlayerCharacter/Input/IMC_Movement.IMC_Movement" (struct))
      (bind _returnvalue_2 (`|CreateWidget` "/Game/HouseEdwards/Blueprints/Interactables/Readables/WBP_ReadableViewer.WBP_ReadableViewer_C" (`GameplayStatics.GetPlayerController` 0)))
      (set `self.w_Widget` _returnvalue_2)
      (`/Game/HouseEdwards/Blueprints/Interactables/Readables/WBP_ReadableViewer.SetTexture` _returnvalue_2 (`self.t_Texture`))
      (`UserWidget.AddToViewport` _returnvalue_2 0)
      (`GameplayStatics.PlaySound2D` "/Game/HouseEdwards/Assets/Audio/AudioAssets/Paper/SC_HandlePaper.SC_HandlePaper" 1.0 1.0 0.0 null null))))

(fn `UserConstructionScript`
  (`parent.UserConstructionScript`)
  (bind _returnvalue (`PrimitiveComponent.CreateDynamicMaterialInstance` (`self.Plane`) 0 "/Game/HouseEdwards/Blueprints/Interactables/Readables/M_Readable.M_Readable" "None"))
  (`MaterialInstanceDynamic.SetTextureParameterValue` _returnvalue "Texture" (`self.t_Texture`)))