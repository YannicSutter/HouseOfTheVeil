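; Base Blueprint for interactable actors, providing a shared Interact entry point with audio feedback.
; Interact checks IsInteractive, then either plays the success sound and calls InteractLogic, or plays only the fail sound.
; InteractLogic is an empty event, leaving the specific behavior to be filled in, presumably by child Blueprints.
; Both sounds play at the actor's location.
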(event `InteractLogic`
  ;[0.15 0.01896 0 0.5] Interact Logic
)

(event `PlaySoundInteractSuccess`
  ;[0 0.02405 0.15 0.5] Interact Sounds
  (`GameplayStatics.PlaySoundAtLocation` (`self.sc_InteractSuccess`) (`self.K2_GetActorLocation`) (struct) 1.0 1.0 0.0 null null null null))

(event `PlaySoundInteractFail`
  ;[0 0.02405 0.15 0.5] Interact Sounds
  (`GameplayStatics.PlaySoundAtLocation` (`self.sc_InteractFail`) (`self.K2_GetActorLocation`) (struct) 1.0 1.0 0.0 null null null null))

(fn `Interact`
  (params (Owner :type "/Game/HouseEdwards/Blueprints/PlayerCharacter/BP_PlayerCharacter Object Reference"))
  (if (`self.bIsInteractive`)
    (`self.PlaySoundInteractSuccess`)
    (`self.InteractLogic`)
    (else
      (`self.PlaySoundInteractFail`))))

(fn `UserConstructionScript`)