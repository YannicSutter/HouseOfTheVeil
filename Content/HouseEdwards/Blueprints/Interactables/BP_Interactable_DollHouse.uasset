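; Doll house interactable that takes the doll the player carries and advances a three-round progression.
; Each round reveals a family doll and clears the player's; the first two unlock the piano and kids' room doors and shift room lights.
; The third plays the guestbook sound and sets BHasAllDolls, but the guestbook activation branch is unreachable because Round never exceeds 3 at its check.
; A separate EndDemo event activates the end-demo trigger.
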(event `self.ReceiveBeginPlay`
  ;[0 0.15 0.1151 0.5] General
  (`parent.ReceiveBeginPlay`)
  (set `self.b_IsActive` true))

(event `self.InteractLogic`
  ;[0.15 0 0.01265 0.5] Interact Logic
  (`parent.InteractLogic`)
  (bind _asbp_player_character (cast `/Game/HouseEdwards/Blueprints/PlayerCharacter/BP_PlayerCharacter` (`GameplayStatics.GetPlayerCharacter` 0)))
  (if (`/Game/HouseEdwards/Blueprints/PlayerCharacter/BP_PlayerCharacter.b_hasDoll` _asbp_player_character)
    (switch `int` (`self.Round`)
      (:`1`
        (`SceneComponent.SetVisibility` (`self.Doll_Father`) true false)
        (`LightComponent.SetIntensity` (`self.Light_Piano`) 1000.0)
        (`GameplayStatics.PlaySound2D` "/Game/HouseEdwards/Assets/Audio/AudioAssets/Door/SC_DoorUnlock.SC_DoorUnlock" 1.0 1.0 0.0 null null)
        (set `/Game/HouseEdwards/Blueprints/Interactables/BP_Interactable_Base.b_IsActive` true (`self.a_DoorPianoRoom`)))
      (:`2`
        (`SceneComponent.SetVisibility` (`self.Doll_Mother`) true false)
        (`LightComponent.SetIntensity` (`self.Light_Piano`) 0.0)
        (`LightComponent.SetIntensity` (`self.Light_Chess`) 1000.0)
        (`GameplayStatics.PlaySound2D` "/Game/HouseEdwards/Assets/Audio/AudioAssets/Door/SC_DoorUnlock.SC_DoorUnlock" 1.0 1.0 0.0 null null)
        (set `/Game/HouseEdwards/Blueprints/Interactables/BP_Interactable_Base.b_IsActive` true (`self.a_DoorKidsRoom`)))
      (:`3`
        (`SceneComponent.SetVisibility` (`self.Doll_Brother`) true false)
        (`LightComponent.SetIntensity` (`self.Light_Chess`) 0.0)
        (`AddComponent|NODE_AddAudioComponent-0`)
        (`GameplayStatics.PlaySound2D` "/Game/HouseEdwards/Assets/Audio/AudioAssets/Paper/SC_GuestBook.SC_GuestBook" 1.0 1.0 0.0 null null)
        (set `self.b_HasAllDolls` true)))
    (set `/Game/HouseEdwards/Blueprints/PlayerCharacter/BP_PlayerCharacter.b_hasDoll` false _asbp_player_character)
    (`StaticMeshComponent.SetStaticMesh` (`/Game/HouseEdwards/Blueprints/PlayerCharacter/BP_PlayerCharacter.Doll` _asbp_player_character) null)
    (if (<= (`self.Round`) 3)
      (set `self.Round` (+ (`self.Round`) 1))
      (else
        (`/Game/HouseEdwards/Blueprints/Interactables/LightSystem/BP_CandleLight.Blink` (`self.a_GuestBookLight`))
        (set `/Game/HouseEdwards/Blueprints/Interactables/BP_Interactable_Base.b_IsActive` true (`self.a_Guestbook`))))))

(event `EndDemo`
  ;[0.15 0 0.01265 0.5] Interact Logic
  (set `/Game/HouseEdwards/Blueprints/Triggers/BP_EndDemoTrigger.b_isActive` true (`self.a_EndDemoTrigger`)))

(fn `UserConstructionScript`
  (`parent.UserConstructionScript`))