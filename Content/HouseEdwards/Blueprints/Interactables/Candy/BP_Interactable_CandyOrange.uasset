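; Orange candy pickup for the HouseEdwards game that adds to the candy score when the player interacts with it.
; It extends a parent interactable, marking itself active on BeginPlay and clearing the success and fail interaction sounds.
; On interaction it runs the parent logic, casts the game mode to GM_Base to increment the candy score, then destroys itself.
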(event `self.ReceiveBeginPlay`
  ;[0 0.1615 0.1313 0.5] General
  (`parent.ReceiveBeginPlay`)
  ;; Candies are always active
  (set `self.b_IsActive` true)
  ;; Sound Settings
  (set `self.sc_InteractSuccess` null)
  (set `self.sc_InteractFail` null))

(event `self.InteractLogic`
  ;[0.15 0.01341 0 0.5] Interact Logic
  (`parent.InteractLogic`)
  (bind _asgm_base (cast `/Game/HouseEdwards/Blueprints/Gamemodes/GM_Base` (`GameplayStatics.GetGameMode`)))
  (`/Game/HouseEdwards/Blueprints/Gamemodes/GM_Base.AddToCandyScore` _asgm_base)
  (`self.K2_DestroyActor`))

(fn `UserConstructionScript`
  (`parent.UserConstructionScript`))