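; BP_CandleLight is an interactable candle fixture with three flickering flame lights, each a BP_Lightflickering child actor.
; On interaction, if the player's lamp is visible and the candle is unlit, it ignites and lerps all three lights, then flags itself as lit.
; A separate Blink event for special candles blinks only the third light and plays a paper sound at the actor's location.
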(event `self.ReceiveBeginPlay`
  ;[0 0.15 0.09994 0.5] General
  (`parent.ReceiveBeginPlay`)
  (set `self.b_IsActive` true))

(event `self.InteractLogic`
  ;[0.15 0 0.01027 0.5] Interact Logic
  (`parent.InteractLogic`)
  (bind _asbp_player_character (cast `/Game/HouseEdwards/Blueprints/PlayerCharacter/BP_PlayerCharacter` (`GameplayStatics.GetPlayerCharacter` 0)))
  (if (`SceneComponent.bVisible` (`/Game/HouseEdwards/Blueprints/PlayerCharacter/BP_PlayerCharacter.Lamp` _asbp_player_character))
    (if (not (`self.b_candleIsLit`))
      (bind _asbp_lightflickering (cast `/Game/HouseEdwards/Assets/EntranceHall/BP_Candle/BP_Lightflickering` (`ChildActorComponent.ChildActor` (`self.LightSource`))))
      (`/Game/HouseEdwards/Assets/EntranceHall/BP_Candle/BP_Lightflickering.IgniteFlame` _asbp_lightflickering)
      (`/Game/HouseEdwards/Assets/EntranceHall/BP_Candle/BP_Lightflickering.LightLerp` _asbp_lightflickering)
      (bind _asbp_lightflickering_2 (cast `/Game/HouseEdwards/Assets/EntranceHall/BP_Candle/BP_Lightflickering` (`ChildActorComponent.ChildActor` (`self.LightSource1`))))
      (`/Game/HouseEdwards/Assets/EntranceHall/BP_Candle/BP_Lightflickering.IgniteFlame` _asbp_lightflickering_2)
      (`/Game/HouseEdwards/Assets/EntranceHall/BP_Candle/BP_Lightflickering.LightLerp` _asbp_lightflickering_2)
      (bind _asbp_lightflickering_3 (cast `/Game/HouseEdwards/Assets/EntranceHall/BP_Candle/BP_Lightflickering` (`ChildActorComponent.ChildActor` (`self.LightSource2`))))
      (`/Game/HouseEdwards/Assets/EntranceHall/BP_Candle/BP_Lightflickering.IgniteFlame` _asbp_lightflickering_3)
      (`/Game/HouseEdwards/Assets/EntranceHall/BP_Candle/BP_Lightflickering.LightLerp` _asbp_lightflickering_3)
      (set `self.b_candleIsLit` true))))

(event `Blink`
  ;[0 0.04271 0.15 0.5] Special Candles
  (bind _asbp_lightflickering (cast `/Game/HouseEdwards/Assets/EntranceHall/BP_Candle/BP_Lightflickering` (`ChildActorComponent.ChildActor` (`self.LightSource2`))))
  (`/Game/HouseEdwards/Assets/EntranceHall/BP_Candle/BP_Lightflickering.Blink` _asbp_lightflickering)
  (`GameplayStatics.PlaySoundAtLocation` "/Game/HouseEdwards/Audio/Interactables/SC_Paper.SC_Paper" (`self.K2_GetActorLocation`) (struct) 1.0 1.0 0.0 null null null null))

(fn `UserConstructionScript`)