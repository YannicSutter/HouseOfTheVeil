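; BP_Interactable_Lamp is an always-active interactable child Blueprint that serves as a lamp pickup for the player.
; BeginPlay marks it active and clears the success and fail interact sounds.
; On interact, it casts the player to BP_PlayerCharacter, reveals that character's existing Lamp and NSFlame components with their children, then destroys itself.
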(event `self.ReceiveBeginPlay`
  ;[0 0.15 0.1012 0.5] General
  (`parent.ReceiveBeginPlay`)
  ;; The lamp is always active
  (set `self.b_IsActive` true)
  ;; Sound Settings
  (set `self.sc_InteractSuccess` null)
  (set `self.sc_InteractFail` null))

(event `self.InteractLogic`
  ;[0.15 0.0112 0 0.5] Interact Logic
  (`parent.InteractLogic`)
  (bind _asbp_player_character (cast `/Game/HouseEdwards/Blueprints/PlayerCharacter/BP_PlayerCharacter` (`GameplayStatics.GetPlayerCharacter` 0)))
  (`SceneComponent.SetVisibility` (`/Game/HouseEdwards/Blueprints/PlayerCharacter/BP_PlayerCharacter.Lamp` _asbp_player_character) true true)
  (`SceneComponent.SetVisibility` (`/Game/HouseEdwards/Blueprints/PlayerCharacter/BP_PlayerCharacter.NS_Flame` _asbp_player_character) true true)
  (`self.K2_DestroyActor`))

(fn `UserConstructionScript`
  (`parent.UserConstructionScript`))