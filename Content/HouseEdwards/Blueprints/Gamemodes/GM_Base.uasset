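; Base game mode that runs the main menu, intro sequence, candy score and puzzle progress flags.
; BeginPlay shows the menu, caches walk positions and totals orange and green candy actors for the maximum score.
; StartGame knocks, opens the double door and walks the player inside via a timeline, then enables vision and the tutorial.
; It also holds test events that submit and fetch scores as JSON over HTTP with an API key.
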(event `self.ReceiveBeginPlay`
  (bind _returnvalue (`GameplayStatics.GetPlayerController` 0))
  (bind _returnvalue_2 (`self.K2_GetActorLocation` (`GameplayStatics.GetPlayerCharacter` 0)))
  ;[0 0.15 0.09806 0.5] General
  ;; Networking stuff
  (`HttpBlueprintFunctionLibrary.AddHeader` (`self.httpRequest`) "x-api-key" (`self.s_api-key`))
  ;; Add Main Menu
  (bind _returnvalue_3 (`|CreateWidget` "/Game/HouseEdwards/Blueprints/UI/WBP_MainMenu.WBP_MainMenu_C"))
  (bind _output_get (set `self.wbp_MainMenu` _returnvalue_3))
  (`UserWidget.AddToViewport` _output_get 0)
  (set `PlayerController.bShowMouseCursor` true _returnvalue)
  (`WidgetBlueprintLibrary.SetInputMode_UIOnlyEx` _returnvalue _output_get)
  ;; Set Game Start locations
  (set `self.v_startLocation` _returnvalue_2)
  (set `self.v_targetLocation` (`KismetMathLibrary.MakeVector` (+ (.x _returnvalue_2) 500.0) (.y _returnvalue_2) (.z _returnvalue_2)))
  ;; Calculate Max Candy Score
  (bind _outactors (`GameplayStatics.GetAllActorsOfClass` "/Game/HouseEdwards/Blueprints/Interactables/Candy/BP_Interactable_CandyOrange.BP_Interactable_CandyOrange_C"))
  (bind _outactors_2 (`GameplayStatics.GetAllActorsOfClass` "/Game/HouseEdwards/Blueprints/Interactables/Candy/BP_Interactable_CandyGreen.BP_Interactable_CandyGreen_C"))
  (set `self.i_maxCandyScore` (+ (`KismetArrayLibrary.Array_Length` _outactors_2) (`KismetArrayLibrary.Array_Length` _outactors))))

(event `AddToCandyScore`
  ;[0.15 0.01408 0 0.5] Candy System
  (set `self.i_Candyscore` (+ (`self.i_Candyscore`) 1))
  (bind _returnvalue (`|CreateWidget` "/Game/HouseEdwards/Blueprints/Interactables/Candy/WBP_CandyScore.WBP_CandyScore_C" (`GameplayStatics.GetPlayerController` 0)))
  (`UserWidget.AddToViewport` _returnvalue 0)
  (`KismetSystemLibrary.Delay` 3.0)
  (`Widget.RemoveFromParent` _returnvalue))

(event `TestHTTPSubmit`
  ;[0 0.04023 0.15 0.5] Testing for API Calls
  (bind (_outjsonstring _returnvalue) (`|StructToJsonString` (make `/Game/HouseEdwards/Blueprints/Interactables/Networking/STRUCT_RequestBody` "submit" (`KismetGuidLibrary.Conv_GuidToString` (`KismetGuidLibrary.NewGuid`)) "10" "TestTest3")))
  (if _returnvalue
    (bind (_outheader _result_body) (`|HttpRequest` (`self.s_URL`) "Post" (`self.httpRequest`) _outjsonstring)
      (:`On Success`
        (bind _outjsonstring_2 (`JsonBlueprintFunctionLibrary.ToString` _result_body))
        (`KismetSystemLibrary.PrintString` _outjsonstring_2))
      (:`On Error`
        (`KismetSystemLibrary.PrintString` "HTTP Request Unsuccessful")))))

(event `TestHTTPGet`
  ;[0 0.04023 0.15 0.5] Testing for API Calls
  (bind (_outjsonstring _returnvalue) (`|StructToJsonString` (make `/Game/HouseEdwards/Blueprints/Interactables/Networking/STRUCT_RequestBody` "get")))
  (if _returnvalue
    (bind (_outheader _result_body) (`|HttpRequest` (`self.s_URL`) "Post" (`self.httpRequest`) _outjsonstring)
      (:`On Success`
        (bind _outjsonstring_2 (`JsonBlueprintFunctionLibrary.ToString` _result_body))
        (`KismetSystemLibrary.PrintString` _outjsonstring_2))
      (:`On Error`
        (`KismetSystemLibrary.PrintString` "HTTP Request Unsuccessful")))))

(event `StartGame`
  ;[0.04297 0 0.15 0.5] Gameflow
  (set `PlayerController.bShowMouseCursor` false (`GameplayStatics.GetPlayerController` 0))
  ;; Door and walking animation
  (bind _outactors (`GameplayStatics.GetAllActorsOfClass` "/Game/HouseEdwards/Blueprints/Interactables/Doors/BP_Interactable_DoubleDoor.BP_Interactable_DoubleDoor_C"))
  (bind _output (`|GetArrayItem` _outactors))
  (`GameplayStatics.PlaySoundAtLocation` "/Game/HouseEdwards/Assets/Audio/AudioAssets/Door/SC_KnockOnDoor.SC_KnockOnDoor" (`self.K2_GetActorLocation` _output) (struct) 1.0 1.0 0.0 null null null null)
  (`KismetSystemLibrary.Delay` 2.0)
  (`/Game/HouseEdwards/Blueprints/Interactables/Doors/BP_Interactable_DoubleDoor.OpenDoor` _output)
  (`KismetSystemLibrary.Delay` (* (`TimelineComponent.GetTimelineLength` (`/Game/HouseEdwards/Blueprints/Interactables/Doors/BP_Interactable_DoubleDoor.ti_OpenDoor` _output)) 0.8))
  (bind _wbp_mainmenu (`self.wbp_MainMenu`)
    (:`then`
      (`Widget.RemoveFromParent` _wbp_mainmenu)
      (bind (_direction _walk) (`Timeline|PlayerWalk` :!via `PlayFromStart`)
        (:`Update`
          (`self.K2_SetActorLocation` (`GameplayStatics.GetPlayerCharacter` 0) (`KismetMathLibrary.VLerp` (`self.v_startLocation`) (`self.v_targetLocation`) _walk) false false))
        (:`Finished`
          (bind _returnvalue (`GameplayStatics.GetActorOfClass` "/Game/HouseEdwards/Blueprints/PlayerCharacter/BP_PlayerCharacter.BP_PlayerCharacter_C"))
          (`/Game/HouseEdwards/Blueprints/PlayerCharacter/BP_PlayerCharacter.Enable VisionCollider` _returnvalue)
          (`WidgetBlueprintLibrary.SetInputMode_GameOnly` (`GameplayStatics.GetPlayerController` 0))
          (bind _returnvalue_2 (`|CreateWidget` "/Game/HouseEdwards/Blueprints/UI/WBP_TutorialUI.WBP_TutorialUI_C"))
          (`UserWidget.AddToViewport` _returnvalue_2 0))
        (:`Close Door`
          (`/Game/HouseEdwards/Blueprints/Interactables/Doors/BP_Interactable_DoubleDoor.CloseDoor` _output))))
    (:`else`)))

(event `SolvedChessPuzzle`
  ;[0.04297 0 0.15 0.5] Gameflow
  (set `self.b_solvedChessPuzzle` true))

(event `SolvedPianoPuzzle`
  ;[0.04297 0 0.15 0.5] Gameflow
  (set `self.b_solvedPianoPuzzle` true))

(fn `UserConstructionScript`)