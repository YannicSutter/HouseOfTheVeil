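; A candle Blueprint for the entrance hall that exposes events to ignite its Niagara flame and animate its CandleLight.
; BeginPlay caches the light's starting intensity, which both timelines scale.
; LightLerp makes the light visible and runs a timeline up to a final snap to that cached intensity, while Blink runs a separate timeline scaled to fifty times it.
; Nothing in this graph calls IgniteFlame, LightLerp or Blink.
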(event `self.ReceiveBeginPlay`
  (set `self.f_maxIntensity` (`LightComponentBase.Intensity` (`self.Candle_Light`))))

(event `IgniteFlame`
  (`ActorComponent.Activate` (`self.NS_Flame`) false))

(event `LightLerp`
  (`SceneComponent.SetVisibility` (`self.Candle_Light`) true true)
  (bind (_direction _intensity) (`Timeline|Intensitylerp` :!via `PlayFromStart`)
    (:`Update`
      (`LightComponent.SetIntensity` (`self.Candle_Light`) (* _intensity (`self.f_maxIntensity`))))
    (:`Finished`
      (`LightComponent.SetIntensity` (`self.Candle_Light`) (`self.f_maxIntensity`)))))

(event `Blink`
  (bind (_direction _alpha) (`Timeline|IntensityBlink` :!via `PlayFromStart`)
    (:`Update`
      (`LightComponent.SetIntensity` (`self.Candle_Light`) (* _alpha (* (`self.f_maxIntensity`) 50.0))))))

(fn `UserConstructionScript`)